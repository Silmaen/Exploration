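; BP_EXP_InventoryItem represents an inventory item stack in Explorer, holding a data table RowName and an Amount.
; Getters look up DT_EXP_ItemInfo by RowName for item info, stackability, max stack and remaining room, printing a message when the row is missing.
; Amount has a simple getter and setter, while OnUse and OnDrop are empty stubs.
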(fn GetInventoryItemInfo
  (bind _rowname (Variables|Default|GetRowName))
  (bind _returnvalue (Utilities|GetDataTableRow "/Game/Explorer/Blueprints/Structs/DataTable/DT_EXP_ItemInfo.DT_EXP_ItemInfo" _rowname)
    (:then
      (return _returnvalue))
    (:RowNotFound
      (Development|PrintString 0 (Utilities|String|Append "Row: " (Utilities|String|ToString(Name) _rowname) " Not found"))
      (return ""))))

(fn GetItemInfo
  (bind _rowname (Variables|Default|GetRowName))
  (bind _returnvalue (Utilities|GetDataTableRow "/Game/Explorer/Blueprints/Structs/DataTable/DT_EXP_ItemInfo.DT_EXP_ItemInfo" _rowname)
    (:then
      (return (.iteminfo _returnvalue)))
    (:RowNotFound
      (Development|PrintString 0 (Utilities|String|Append "Row: " (Utilities|String|ToString(Name) _rowname) " Not found"))
      (return ""))))

(fn GetCanStack
  (bind _rowname (Variables|Default|GetRowName))
  (bind _returnvalue (Utilities|GetDataTableRow "/Game/Explorer/Blueprints/Structs/DataTable/DT_EXP_ItemInfo.DT_EXP_ItemInfo" _rowname)
    (:then
      (return (.canstack? _returnvalue)))
    (:RowNotFound
      (Development|PrintString 0 (Utilities|String|Append "Row: " (Utilities|String|ToString(Name) _rowname) " Not found"))
      (return false))))

(fn GetMaxStackAmount
  (bind _rowname (Variables|Default|GetRowName))
  (bind _returnvalue (Utilities|GetDataTableRow "/Game/Explorer/Blueprints/Structs/DataTable/DT_EXP_ItemInfo.DT_EXP_ItemInfo" _rowname)
    (:then
      (return (.maxstackamount _returnvalue)))
    (:RowNotFound
      (Development|PrintString 0 (Utilities|String|Append "Row: " (Utilities|String|ToString(Name) _rowname) " Not found"))
      (return -1))))

(fn GetRoomOnstack
  (bind _rowname (Variables|Default|GetRowName))
  (bind _returnvalue (Utilities|GetDataTableRow "/Game/Explorer/Blueprints/Structs/DataTable/DT_EXP_ItemInfo.DT_EXP_ItemInfo" _rowname)
    (:then
      (return (- (.maxstackamount _returnvalue) (Variables|Default|GetAmount))))
    (:RowNotFound
      (Development|PrintString 0 (Utilities|String|Append "Row: " (Utilities|String|ToString(Name) _rowname) " Not found"))
      (return -1))))

(fn OnUse)

(fn OnDrop)

(fn GetAmount
  (return (Variables|Default|GetAmount)))

(fn SetAmount
  (params (Amount :type Integer))
  (Variables|Default|SetAmount Amount))