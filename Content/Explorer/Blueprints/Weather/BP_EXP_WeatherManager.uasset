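; Weather manager actor that runs a day/night cycle with an in-game clock, dynamic sky and fluctuating world temperature.
; Construction converts start time to elapsed seconds and sets up the sky material, previewing the initial sun position.
; Each tick advances time and rotates the sun by day fraction, elevation and north angle; sun height samples color curves for sky and lights.
; A looping named-function timer is started for curve-based temperature updates.
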(event EventBeginPlay
  (Temperature|StartTemperatureFluctuationTimer))

(event EventTick
  (params (DeltaSeconds :type Float%20%28single-precision%29))
  (Utilities|FlowControl|Sequence
    (:then_0
      (DayNightCycle|UpdateSunPosition))
    (:then_1
      (Time|UpdateElapsedTime))
    (:then_2
      (Time|UpdateCurrentTime))))

(fn ConstructionScript
  ;[1 1 1] TimeInitialization
  (Variables|Time|SetSecondsPerDay (* (Variables|Time|GetMinutesPerDay) 6e+01))
  (Time|SetElapsedTimeBasedonStartTime)
  (Variables|Time|SetCurrentTime (Variables|Time|GetStartTime))
  ;[1 1 1] Initial position of all component is reset to 0
  (Transformation|SetWorldLocation (Variables|Default|GetSky_Mesh) "0, 0, 0" false false)
  ;[1 1 1] Sky and Sun
  (bind _returnvalue (Rendering|Material|CreateDynamicMaterialInstance (Variables|Default|GetSky_Mesh) 0 (Variables|DayNightCycle|Sky|GetBaseSkyMaterial) "None" :!class /Script/Engine.PrimitiveComponent))
  (Variables|DayNightCycle|Sky|SetSkyMaterial _returnvalue)
  (DayNightCycle|UpdateSunPosition)
  ;;[1 1 1] Constant material parameters
  (Rendering|Material|SetScalarParameterValue (Variables|DayNightCycle|Sky|GetSkyMaterial) "Cloud speed" (Variables|DayNightCycle|Sky|GetCloudSpeed) :!class /Script/Engine.MaterialInstanceDynamic)
  (Rendering|Material|SetScalarParameterValue (Variables|DayNightCycle|Sky|GetSkyMaterial) "Sun brightness" (Variables|DayNightCycle|Sun|GetSunBrightness) :!class /Script/Engine.MaterialInstanceDynamic)
  (Rendering|Material|SetScalarParameterValue (Variables|DayNightCycle|Sky|GetSkyMaterial) "Cloud opacity" (Variables|DayNightCycle|Sky|GetCloudOpacity) :!class /Script/Engine.MaterialInstanceDynamic)
  (Rendering|Material|SetScalarParameterValue (Variables|DayNightCycle|Sky|GetSkyMaterial) "Stars brightness" (Variables|DayNightCycle|Sky|GetStarsBrightness) :!class /Script/Engine.MaterialInstanceDynamic)
  (Rendering|Material|SetScalarParameterValue (Variables|DayNightCycle|Sky|GetSkyMaterial) "Sun Radius" (Variables|DayNightCycle|Sun|GetSunRadius) :!class /Script/Engine.MaterialInstanceDynamic))

(fn SetElapsedTimeBasedonStartTime
  (Variables|Time|SetElapsedTime (* (CallFunction|GetTimeasSeconds (Variables|Time|GetStartTime)) (/ (Variables|Time|GetSecondsPerDay) 8.64e+04))))

(fn UpdateSunPosition
  (bind _sunheight (Variables|DayNightCycle|Sun|GetsunHeight))
  (bind _sky_light (Variables|Default|GetSky_Light))
  (bind _sunheight_2 (Variables|DayNightCycle|Sun|GetsunHeight))
  (bind _skymaterial (Variables|DayNightCycle|Sky|GetSkyMaterial))
  (DayNightCycle|SetSunDirection)
  (Rendering|Material|SetVectorParameterValue _skymaterial "Light direction" (Math|Conversions|ToLinearColor(Vector) (Math|Rotator|GetRotationXVector (Transformation|GetWorldRotation (Variables|Default|GetSun_Light)))) :!class /Script/Engine.MaterialInstanceDynamic)
  (Rendering|Material|SetVectorParameterValue _skymaterial "Sun color" (Math|Curves|GetLinearColorValue (Variables|DayNightCycle|Sun|GetSunColorCurve) _sunheight) :!class /Script/Engine.MaterialInstanceDynamic)
  (Rendering|Material|SetVectorParameterValue _skymaterial "Horizon color" (Math|Curves|GetLinearColorValue (Variables|DayNightCycle|Sky|GetHorizonColorCurve) _sunheight) :!class /Script/Engine.MaterialInstanceDynamic)
  (Rendering|Material|SetVectorParameterValue _skymaterial "Zenith color" (Math|Curves|GetLinearColorValue (Variables|DayNightCycle|Sky|GetZenithColorCurve) _sunheight) :!class /Script/Engine.MaterialInstanceDynamic)
  (Rendering|Material|SetVectorParameterValue _skymaterial "Cloud color" (Math|Curves|GetLinearColorValue (Variables|DayNightCycle|Sky|GetCloudColorCurve) _sunheight) :!class /Script/Engine.MaterialInstanceDynamic)
  (Rendering|Material|SetScalarParameterValue _skymaterial "Horizon falloff" (Math|Float|Lerp 3.0 8.0 (Math|Float|Absolute(Float) _sunheight)) :!class /Script/Engine.MaterialInstanceDynamic)
  (Rendering|Material|SetScalarParameterValue _skymaterial "Sun height" (Math|Float|SelectFloat (Math|Float|Absolute(Float) _sunheight) 0.0 (< _sunheight 0.0)) :!class /Script/Engine.MaterialInstanceDynamic)
  (Rendering|Components|Light|SetLightColor _sky_light (Math|Curves|GetLinearColorValue (Variables|DayNightCycle|Sky|GetSkyLightColorCurve) _sunheight_2))
  (Rendering|Components|Light|SetIntensity _sky_light (+ (* (Math|Float|Clamp(Float) (+ (* _sunheight_2 -1.0) 0.1)) 3e+01) 0.2)))

(fn GetFractionOfDay
  (return (/ (Variables|Time|GetElapsedTime) (Variables|Time|GetSecondsPerDay))))

(fn UpdateElapsedTime
  (Variables|Time|SetElapsedTime (+ (Variables|Time|GetElapsedTime) (Utilities|Time|GetWorldDeltaSeconds))))

(fn UpdateCurrentTime
  (Variables|Time|SetCurrentTime (Time|DetermineCurrentTime)))

(fn DetermineCurrentTime
  (bind _dayfraction (Time|GetFractionOfDay))
  (return (Utilities|Struct|MakeS_EXP_Time (Math|Float|Truncate _dayfraction) (Math|Float|Truncate (* (Math|Float|%(Float) _dayfraction 1.0) 24.0)) (Math|Float|Truncate (Math|Float|%(Float) (* _dayfraction 1.44e+03) 6e+01)))))

(fn DetermineifNight
  (bind _currenttime (Variables|Time|GetCurrentTime))
  (bind _output_get (Variables|DayNightCycle|SetIsNight? (or (> (.hours _currenttime) (Variables|Time|GetSunUpTime)) (>= (.hours _currenttime) (Variables|Time|GetSunDownTime)))))
  (return _output_get))

(fn StartTemperatureFluctuationTimer
  (Utilities|Time|SetTimerbyFunctionName self (Variables|Temperature|GetUpdateTemperatureTimerName) (Variables|Temperature|GetTemperatureUpdateRate) true))

(fn UpdateWordTemperature
  (Variables|Temperature|SetFinalWorldTemperature (+ (* (Math|Curves|GetFloatValue (Variables|Temperature|GetTempFluctuationCurve) (Math|Float|%(Float) (Time|GetFractionOfDay) 1.0)) (Variables|Temperature|GetWorldTemperatureVariation)) (Variables|Temperature|GetBaseWorldTemperature))))

(fn SetSunDirection
  ;[1 1 1] Light Rotation
  (Transformation|SetWorldRotation (Variables|Default|GetSun_Light) (Math|Rotator|MakeRotfromX (Math|Vector|RotateVector (Math|Vector|RotateVector (Math|Vector|RotateVector "1.000000, 0, 0" (Math|Rotator|MakeRotator 0.0 (+ (* (Time|GetFractionOfDay) -3.6e+02) 9e+01) 0.0)) (Math|Rotator|MakeRotator (- (Variables|DayNightCycle|Sun|GetElevation) 9e+01) 0.0 0.0)) (Math|Rotator|MakeRotator 0.0 0.0 (Variables|DayNightCycle|Sun|GetNorthAngle)))) false false)
  ;[1 1 1] ComputeSunHeight Factor
  (Variables|DayNightCycle|Sun|SetsunHeight (Math|Float|MapRangeUnclamped (.Pitch (Math|Rotator|BreakRotator (Transformation|GetWorldRotation (Variables|Default|GetSun_Light)))) 0.0 -9e+01 0.0 1.0))
  ;[1 1 1] Set Sun Light Color
  (Rendering|Components|Light|SetLightColor (Variables|Default|GetSun_Light) (Math|Curves|GetLinearColorValue (Variables|DayNightCycle|Sun|GetSunColorCurve) (Variables|DayNightCycle|Sun|GetsunHeight)) true))