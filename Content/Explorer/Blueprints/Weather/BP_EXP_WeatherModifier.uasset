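; Weather modifier volume actor that alters the temperature felt by BP_EXP_Pawn inside a box area.
; The construction script sizes the box from its BoxExtent variable.
; Begin overlap calls ApplyTempModifier on the pawn with an optional world temperature override and an additional area modifier.
; End overlap calls it again with the override cleared and the area modifier minus one, rather than its negation.
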(event OnComponentBeginOverlap(Volume)
  (params (OverlappedComponent :type Primitive%20Component%20Object%20Reference) (OtherActor :type Actor%20Object%20Reference) (OtherComp :type Primitive%20Component%20Object%20Reference) (OtherBodyIndex :type Integer) (bFromSweep :type Boolean) (SweepResult :type Hit%20Result%20Structure%20%28by%20ref%29))
  (bind _asbp_exp_pawn (Utilities|Casting|CastToBP_EXP_Pawn OtherActor))
  (Default|ApplyTempModifier _asbp_exp_pawn (Variables|Temperature|GetOverideLocalWorldTemp?) (Variables|Temperature|GetOverridenWorldTemp) (Variables|Temperature|GetAreaTempModifier)))

(event OnComponentEndOverlap(Volume)
  (params (OverlappedComponent :type Primitive%20Component%20Object%20Reference) (OtherActor :type Actor%20Object%20Reference) (OtherComp :type Primitive%20Component%20Object%20Reference) (OtherBodyIndex :type Integer))
  (bind _asbp_exp_pawn (Utilities|Casting|CastToBP_EXP_Pawn OtherActor))
  (Default|ApplyTempModifier _asbp_exp_pawn false 0.0 (- (Variables|Temperature|GetAreaTempModifier) 1.0)))

(fn ConstructionScript
  (Components|Box|SetBoxExtent (Variables|Default|GetVolume) (Variables|Geometry|GetBoxExtent) true))