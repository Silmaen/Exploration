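; Blueprint function library for the Explorer game's day, hour and minute time struct.
; It converts times to and from seconds, which GetDeltaTime uses to return the absolute gap between two times as a struct.
; It also formats 12 or 24 hour clock text and gives the elapsed fraction of a day.
; SetTimeBySecond does not subtract whole days when computing minutes, so multi-day values yield oversized minutes.
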(fn GetTimeasSeconds
  (params (Time :type S%20EXP%20Time%20Structure%20%28by%20ref%29))
  (bind (_days _hours _minutes) (Utilities|Struct|BreakS_EXP_Time Time))
  (return (+ (* _days 86400) (* _hours 3600) (* _minutes 60))))

(fn TimeasText
  (params (Time :type S%20EXP%20Time%20Structure) (TypeOfClock :type E_EXP_ClockType%20Enum :default "NewEnumerator0"))
  (bind (_days _hours _minutes) (Utilities|Struct|BreakS_EXP_Time Time))
  (bind (_days_2 _hours_2 _minutes_2) (Utilities|Struct|BreakS_EXP_Time Time))
  (bind _returnvalue (Math|Integer|%(Integer) _hours_2 12))
  (switch Utilities|FlowControl|Switch|SwitchonE_EXP_ClockType TypeOfClock
    (:NewEnumerator0
      (return (Utilities|Text|FormatText "Day {Days}, {hours}:{Minutes} {AM/PM}" _days_2 (Utilities|Text|ToText(Integer) (select (< _returnvalue 1) 12 _returnvalue) false true 2 2) (Utilities|Text|ToText(Integer) _minutes_2 false true 2 2) (select (< _hours_2 12) "AM" "PM"))))
    (:NewEnumerator1
      (return (Utilities|Text|FormatText "Day {Days}, {hours}:{Minutes}" _days (Utilities|Text|ToText(Integer) _hours false true 2 2) (Utilities|Text|ToText(Integer) _minutes false true 2 2))))))

(fn SetTimebySecond
  (params (Seconds :type Float%20%28single-precision%29))
  (bind _returnvalue (/ Seconds 8.64e+04))
  (bind _returnvalue_2 (Math|Float|Truncate _returnvalue))
  (bind _returnvalue_3 (* _returnvalue_2 8.64e+04))
  (bind _returnvalue_4 (- Seconds _returnvalue_3))
  (bind _returnvalue_5 (/ _returnvalue_4 3.6e+03))
  (bind _returnvalue_6 (Math|Float|Truncate _returnvalue_5))
  (return (Utilities|Struct|MakeS_EXP_Time _returnvalue_2 _returnvalue_6 (Math|Float|Truncate (/ (- Seconds (* _returnvalue_6 3.6e+03)) 6e+01)))))

(fn GetDeltaTime
  (params (StartTime :type S%20EXP%20Time%20Structure) (EndTime :type S%20EXP%20Time%20Structure))
  (return (CallFunction|SetTimebySecond (Math|Conversions|ToFloat(Integer) (Math|Integer|Absolute(Integer) (- (CallFunction|GetTimeasSeconds EndTime) (CallFunction|GetTimeasSeconds StartTime)))))))

(fn GetDayFraction
  (params (Date :type S%20EXP%20Time%20Structure))
  (return (/ (Math|Conversions|ToFloat(Integer) (CallFunction|GetTimeasSeconds (Utilities|Struct|MakeS_EXP_Time 0 (.hours Date) (.minutes Date)))) 8.64e+04)))