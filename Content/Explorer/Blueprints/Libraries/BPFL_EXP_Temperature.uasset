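; Blueprint function library of temperature unit conversion helpers for the Explorer content.
; It converts Fahrenheit to Celsius and Celsius to Fahrenheit with the standard linear formulas.
; ToCelsius switches on a temperature unit enum, passing Celsius input through unchanged and converting Fahrenheit input with its own inline copy of the formula.
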(fn FahrenheittoCelsius
  (params (Temperature%20%28Fahrenheit%29 :type Float%20%28single-precision%29))
  (return (* (- Temperature%20%28Fahrenheit%29 32.0) (/ 5.0 9.0))))

(fn CelsiustoFahrenheit
  (params (Temperature%20%28Celsius%29 :type Float%20%28single-precision%29))
  (return (+ (* Temperature%20%28Celsius%29 (/ 9.0 5.0)) 32.0)))

(fn ToCelsius
  (params (TempUnit :type E_EXP_TemperatureType%20Enum :default "NewEnumerator0") (Temperature%20%28input%29 :type Float%20%28single-precision%29))
  (switch Utilities|FlowControl|Switch|SwitchonE_EXP_TemperatureType TempUnit
    (:NewEnumerator0
      (return Temperature%20%28input%29))
    (:NewEnumerator1
      (return (* (- Temperature%20%28input%29 32.0) (/ 5.0 9.0))))))