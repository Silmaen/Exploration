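; BP_ElevatorDoor is a per-floor elevator door with a call button that sends its linked elevator to that floor.
; OpenDoor and CloseDoor play the Opening timeline forward or in reverse unless locked, sliding interior and exterior panels through DoorPosition.
; The construction script applies the Open and Locked state, then configures the child-actor BP_Button with sign and floor number.
; ButtonPushed calls the elevator, or resets the button if it is already there.
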(event Custom|OpenDoor
  (if (not (Variables|State|GetLocked?))
    (if (not (Variables|State|GetOpen?))
      (Variables|State|SetMoving? true)
      (bind _opening (Timeline|Opening PlayFromStart)
        (:Update
          (CallFunction|DoorPosition _opening))
        (:Finished
          (Variables|State|SetMoving? false)
          (Variables|State|SetOpen? (not (Variables|State|GetOpen?))))))))

(event Custom|CloseDoor
  (if (not (Variables|State|GetLocked?))
    (if (Variables|State|GetOpen?)
      (Variables|State|SetMoving? true)
      (bind _opening (Timeline|Opening ReverseFromEnd)
        (:Update
          (CallFunction|DoorPosition _opening))
        (:Finished
          (Variables|State|SetMoving? false)
          (Variables|State|SetOpen? (not (Variables|State|GetOpen?))))))))

(event EventBeginPlay)

(event Collision|EventActorBeginOverlap
  (params (OtherActor :type Actor%20Object%20Reference)))

(event EventTick
  (params (DeltaSeconds :type Float%20%28single-precision%29)))

(fn ConstructionScript
  (Utilities|FlowControl|Sequence
    (:then_0
      ;[1 1 1] Update state
      (if (Variables|State|GetLocked?)
        (Variables|State|SetOpen? false)))
    (:then_1
      ;[1 1 1] Update door position
      (CallFunction|DoorPosition (select (Variables|State|GetOpen?) 1.0 0.0)))
    (:then_2
      ;[1 1 1] Setup button
      (bind _asbp_button (Utilities|Casting|CastToBP_Button (Variables|/Script/Engine.ChildActorComponent|GetChildActor (Variables|Default|GetButton)))
        (:then
          (bind _output_get (Variables|Components|SetTrueButton _asbp_button))
          (Default|SetParent _output_get true self)
          (Variables|/Game/Explorer/Blueprints/Actors/elevator/BP_Button.BP_Button_C|SetToggle? _output_get true)
          (Default|SetSign _output_get "/Game/Explorer/Blueprints/Actors/elevator/T_ElevatorCall.T_ElevatorCall")
          (Default|SetFloorNumber _output_get (Variables|State|GetfloorIndex)))
        (:CastFailed
          (Development|PrintString "Error: DoorButton is not attached correctly"))))))

(fn DoorPosition
  (params (Amount :type Float%20%28single-precision%29))
  (bind _openingamount (Variables|State|GetOpeningAmount))
  (bind _returnvalue (* Amount _openingamount))
  (bind _returnvalue_2 (* _returnvalue -1.0))
  (Transformation|SetRelativeLocation (Variables|Default|GetDoorExtRight) (Math|Vector|MakeVector (+ _returnvalue 416.0) 0.0 0.0) false false)
  (Transformation|SetRelativeLocation (Variables|Default|GetDoorExtLeft) (Math|Vector|MakeVector _returnvalue_2 0.0 0.0) false false)
  (Transformation|SetRelativeLocation (Variables|Default|GetDoorIntRight) (Math|Vector|MakeVector _returnvalue_2 0.0 0.0) false false)
  (Transformation|SetRelativeLocation (Variables|Default|GetDoorIntLeft) (Math|Vector|MakeVector _returnvalue_2 0.0 0.0) false false))

(fn ButtonPushed
  (bind _floorindex (Variables|State|GetfloorIndex))
  (Utilities|IsValid (Variables|Components|GetUsageElevator)
    (:Is%20Valid
      (if (Variables|/Game/Explorer/Blueprints/Actors/elevator/BP_Button.BP_Button_C|GetState (Variables|Components|GetTrueButton))
        (if (== (Variables|/Game/Explorer/Blueprints/Actors/elevator/BP_Elevator.BP_Elevator_C|GetCurrentFloor (Variables|Components|GetUsageElevator)) _floorindex)
          (Default|ResetButton (Variables|Components|GetTrueButton))
          (else
            (Default|GotoFloor (Variables|Components|GetUsageElevator) _floorindex)))))))

(fn ResetButton
  (Default|ResetButton (Variables|Components|GetTrueButton)))