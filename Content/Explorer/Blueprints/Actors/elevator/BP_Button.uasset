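; Elevator button actor that shows a floor number and notifies its parent panel when interacted with.
; Interaction flips the state only in toggle mode, then always updates appearance and calls ButtonPushed on a valid ParentPanel.
; State drives a glow parameter on dynamic materials for the button and text, plus a slight pressed-in offset.
; ResetButton clears the state without notifying the panel, and SetFloorNumber sets the label.
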(event EventInteraction
  (params (CharacterReference :type BP%20EXP%20Pawn%20Object%20Reference))
  (if (Variables|ButtonProperties|GetToggle?)
    (Variables|ButtonProperties|SetState (not (Variables|ButtonProperties|GetState))))
  (CallFunction|OnStateChange))

(fn ConstructionScript
  (bind _button (Variables|Default|GetButton))
  (bind _floortext (Variables|Default|GetFloorText))
  (Variables|ButtonProperties|SetInitialPosition (Transformation|GetRelativeTransform (Variables|Default|GetButton)))
  (bind _returnvalue (Rendering|Material|CreateDynamicMaterialInstance _button 0 (Rendering|Material|GetMaterial _button 0) "None" :!class /Script/Engine.PrimitiveComponent))
  (Variables|Components|SetButtonMaterial _returnvalue)
  (bind _returnvalue_2 (Rendering|Material|CreateDynamicMaterialInstance _floortext 0 (Rendering|Material|GetMaterial _floortext 0) "None" :!class /Script/Engine.PrimitiveComponent))
  (Variables|Components|SetTextMaterial _returnvalue_2))

(fn OnStateChange
  (bind _parentpanel (Variables|ButtonProperties|GetParentPanel))
  (CallFunction|ApearenceUpdate)
  (Utilities|IsValid _parentpanel
    (:Is%20Valid
      (Default|ButtonPushed _parentpanel))))

(fn ResetButton
  (Variables|ButtonProperties|SetState false)
  (CallFunction|ApearenceUpdate))

(fn ApearenceUpdate
  (bind _state (Variables|ButtonProperties|GetState))
  (bind _glowingparametername (Variables|ButtonProperties|GetGlowingParameterName))
  (bind _returnvalue (select _state 1.0 0.0))
  (Rendering|Material|SetScalarParameterValue (Variables|Components|GetButtonMaterial) _glowingparametername _returnvalue :!class /Script/Engine.MaterialInstanceDynamic)
  (Rendering|Material|SetScalarParameterValue (Variables|Components|GetTextMaterial) _glowingparametername _returnvalue :!class /Script/Engine.MaterialInstanceDynamic)
  (Transformation|SetRelativeLocation (Variables|Default|GetButton) (select _state "-0.010000, 0, 0" "0, 0, 0") false false))

(fn SetFloorNumber
  (params (FloorNumber :type Integer))
  (bind _output_get (Variables|ButtonProperties|SetFloorNumber FloorNumber))
  (Rendering|Components|TextRender|SetText (Variables|Default|GetFloorText) (Utilities|Text|ToText(Integer) _output_get false true 1 2)))