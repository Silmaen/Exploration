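; Elevator button panel that sends floor requests to its linked elevator.
; The construction script computes a clamped row and column grid, scales the panel to fit and spawns inverse-scaled BP_Button child actors, each given a floor number and parent reference.
; ButtonPushed calls GoToFloor for each active button, resetting any matching the current floor.
; ResetFloorButton clears the buttons for a given floor.
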(event EventBeginPlay)

(event Collision|EventActorBeginOverlap
  (params (OtherActor :type Actor%20Object%20Reference)))

(event EventTick
  (params (DeltaSeconds :type Float%20%28single-precision%29)))

(fn ConstructionScript
  (bind (_numberofcolumns _numberofrows) (CallFunction|DetermineRowsColumns))
  (bind _basescale (LocalVariables|GetBaseScale))
  (bind _basebtnoffset (Variables|Geometry|GetBaseBtnOffset))
  (Utilities|FlowControl|Sequence
    (:then_0
      ;[1 1 1] Colomns & Rows computation
      (bind _output_get (LocalVariables|SetNumberOfColumn _numberofcolumns))
      (bind _output_get_2 (LocalVariables|SetNumberOfRows _numberofrows))
      ;[1 1 1] Button intial offset
      (LocalVariables|SetButtonPositionOffset (Math|Vector|MakeVector (.x _basebtnoffset) (+ (* _output_get (.y _basebtnoffset)) (* (- _output_get 1) (* (* (Variables|Geometry|GetBtnHorizontalSpacing) 0.5) (select (Variables|Geometry|GetLeftRight?) -1.0 1.0)))) (+ (* _output_get_2 (.z _basebtnoffset)) (* (- _output_get_2 1) (* (* (Variables|Geometry|GetBtnVerticalSpacing) 0.5) (select (Variables|Geometry|GetBottomUp?) 1.0 -1.0)))))))
    (:then_1
      ;[1 1 1] SCale the panel to fit needed space for buttons
      (Transformation|SetRelativeScale3D (Variables|Default|GetPanel) (Math|Vector|MakeVector (.x _basescale) (* (LocalVariables|GetNumberOfColumn) (.y _basescale)) (* (LocalVariables|GetNumberOfRows) (.z _basescale))))
      (bind _output_get_3 (LocalVariables|SetInverseScale (Math|Vector|MakeVector (/ 1.0 (.x _basescale)) (/ 1.0 (* (LocalVariables|GetNumberOfColumn) (.y _basescale))) (/ 1.0 (* (LocalVariables|GetNumberOfRows) (.z _basescale))))))
      (LocalVariables|SetButtonPositionOffset (* _output_get_3 (LocalVariables|GetButtonPositionOffset))))
    (:then_2
      ;[1 1 1] ButtonCreationLoop
      (for _index (range 1 (Variables|Geometry|GetNumberOfButton))
        ;;[1 1 1] create the button
        (bind _returnvalue (AddComponent|AddChildActorComponent false (Math|Transform|MakeTransform (- (* (LocalVariables|GetInverseScale) (Math|Vector|MakeVector 0.0 (* (Math|Integer|%(Integer) (- _index 1) (LocalVariables|GetNumberOfColumn)) (* (Variables|Geometry|GetBtnHorizontalSpacing) (select (Variables|Geometry|GetLeftRight?) -1.0 1.0))) (* (/ (- _index 1) (LocalVariables|GetNumberOfColumn)) (* (Variables|Geometry|GetBtnVerticalSpacing) (select (Variables|Geometry|GetBottomUp?) 1.0 -1.0))))) (LocalVariables|GetButtonPositionOffset)) "0, 0, 0" (* (LocalVariables|GetInverseScale) (Variables|Geometry|GetGlobal%20%20button%20scale)))))
        (ChildActorComponent|SetChildActorClass _returnvalue "/Game/Explorer/Blueprints/Actors/elevator/BP_Button.BP_Button_C")
        (bind _asbp_button (Utilities|Casting|CastToBP_Button (Variables|/Script/Engine.ChildActorComponent|GetChildActor _returnvalue)))
        (Utilities|Array|Add (Variables|Components|GetButtonList) _asbp_button)
        (Variables|/Game/Explorer/Blueprints/Actors/elevator/BP_Button.BP_Button_C|SetParentPanel _asbp_button self)
        (Variables|/Game/Explorer/Blueprints/Actors/elevator/BP_Button.BP_Button_C|SetToggle? _asbp_button true)
        (Default|SetFloorNumber _asbp_button (Utilities|Array|Get(acopy) (Variables|Geometry|GetFloorsIndex) (- _index 1)))))))

(fn DetermineRowsColumns
  (bind _numberofbutton (Variables|Geometry|GetNumberOfButton))
  (bind _columnnumber (Variables|Geometry|GetColumnNumber))
  (bind _returnvalue (Math|Integer|Clamp(Integer) _columnnumber 1 _numberofbutton))
  (return _returnvalue (+ (/ _numberofbutton _returnvalue) (select (> (Math|Integer|%(Integer) _numberofbutton _returnvalue) 0) 1 0))))

(fn ButtonPushed
  (Utilities|IsValid (Variables|Components|GetUsageElevator)
    (:Is%20Valid
      (for (_array_element _array_index) (Variables|Components|GetButtonList)
        (if (Variables|/Game/Explorer/Blueprints/Actors/elevator/BP_Button.BP_Button_C|GetState _array_element)
          (if (== (Variables|/Game/Explorer/Blueprints/Actors/elevator/BP_Elevator.BP_Elevator_C|GetCurrentFloor (Variables|Components|GetUsageElevator)) (Utilities|Array|Get(acopy) (Variables|Geometry|GetFloorsIndex) _array_index))
            (Default|ResetButton _array_element)
            (else
              (Default|GotoFloor (Variables|Components|GetUsageElevator) (Utilities|Array|Get(acopy) (Variables|Geometry|GetFloorsIndex) _array_index)))))))))

(fn ResetFloorButton
  (params (Floor :type Integer))
  (for (_array_element _array_index) (Variables|Geometry|GetFloorsIndex)
    (if (== Floor _array_element)
      (Default|ResetButton (Utilities|Array|Get(acopy) (Variables|Components|GetButtonList) _array_index)))))