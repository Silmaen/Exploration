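; Elevator actor that moves its cage vertically between a list of floor altitudes when a target floor is requested.
; Construction script links the child button panel, clamps the starting floor, snaps the cage to it and adds a billboard per floor.
; GoToFloor starts a looping timer for stepped movement at a capped speed, without easing.
; On arrival the timer clears, the cage snaps, and internal and exterior panels reset that floor's button.
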(fn ConstructionScript
  (bind _elevatorfloorcage (Variables|Default|GetElevatorFloorCage))
  (bind _elevatorfloorcage_2 (Variables|Default|GetElevatorFloorCage))
  (bind _relativelocation (Variables|/Script/Engine.SceneComponent|GetRelativeLocation _elevatorfloorcage_2))
  (bind _relativelocation_2 (Variables|/Script/Engine.SceneComponent|GetRelativeLocation _elevatorfloorcage))
  (Utilities|FlowControl|Sequence
    (:then_0
      ;[1 1 1] Link the internal button panel
      (Variables|/Game/Explorer/Blueprints/Actors/elevator/BP_ButtonPanel.BP_ButtonPanel_C|SetUsageElevator (.AsBP%20Button%20Panel (Utilities|Casting|CastToBP_ButtonPanel (Variables|/Script/Engine.ChildActorComponent|GetChildActor (Variables|Default|GetCommand)))) self))
    (:then_1
      ;[1 1 1] Clamp the current floor
      (Variables|Elevetor|SetCurrentFloor (Math|Integer|Clamp(Integer) (Variables|Elevetor|GetCurrentFloor) 0 (- (Utilities|Array|Length (Variables|Elevetor|GetFloorAltitudes)) 1))))
    (:then_2
      ;[1 1 1] Add sprite to materialize floors in editor
      (for _array_element (Variables|Elevetor|GetFloorAltitudes)
        (bind _returnvalue (AddComponent|AddBillboardComponent false (Math|Transform|MakeTransform (Math|Vector|MakeVector (.x _relativelocation_2) (.y _relativelocation_2) _array_element) "0, 0, 0" "1,1,1")))
        (Variables|/Script/Engine.BillboardComponent|SetSprite _returnvalue "/Engine/EditorResources/Waypoint.Waypoint")))
    (:then_3
      ;[1 1 1] Position the elevator to the current floor
      (if (> (Utilities|Array|Length (Variables|Elevetor|GetFloorAltitudes)) 0)
        (Transformation|SetRelativeLocation (Variables|Default|GetElevatorFloorCage) (Math|Vector|MakeVector (.x _relativelocation) (.y _relativelocation) (Utilities|Array|Get(acopy) (Variables|Elevetor|GetFloorAltitudes) (Variables|Elevetor|GetCurrentFloor))) false false)))))

(fn GotoFloor
  (params (TargetedFloor :type Integer))
  (bind _output_get (Variables|Elevetor|SetTargetedFloor TargetedFloor))
  (if (!= _output_get (Variables|Elevetor|GetCurrentFloor))
    (Utilities|Time|SetTimerbyFunctionName self (Variables|Elevetor|GetMoveFunctionTimer) (Variables|Elevetor|GetPositionUpdateRate) true)))

(fn AtFloor
  (bind _currentfloor (Variables|Elevetor|GetCurrentFloor))
  (Default|ResetFloorButton (.AsBP%20Button%20Panel (Utilities|Casting|CastToBP_ButtonPanel (Variables|/Script/Engine.ChildActorComponent|GetChildActor (Variables|Default|GetCommand)))) _currentfloor)
  (for _array_element (Variables|Elevetor|GetExteriorButonPanel)
    (Default|ResetFloorButton _array_element _currentfloor)))

(fn MoveElevator
  (bind _flooraltitudes (Variables|Elevetor|GetFloorAltitudes))
  (bind _elevatorfloorcage (Variables|Default|GetElevatorFloorCage))
  (bind _relativelocation (Variables|/Script/Engine.SceneComponent|GetRelativeLocation _elevatorfloorcage))
  (bind _output_get (LocalVariables|SetStartingAltitude (Utilities|Array|Get(acopy) _flooraltitudes (Variables|Elevetor|GetCurrentFloor))))
  (bind _output_get_2 (LocalVariables|SetDestinationAltitude (Utilities|Array|Get(acopy) _flooraltitudes (Variables|Elevetor|GetTargetedFloor))))
  (bind _output_get_3 (LocalVariables|SetCurrentAltitude (.z _relativelocation)))
  (if (< (Math|Float|Absolute(Float) (- (+ _output_get_3 (* (Math|Float|Clamp(Float) (* (Variables|Elevetor|GetElevatorMaxSpeed) (Variables|Elevetor|GetPositionUpdateRate)) 0.0 (Math|Float|Absolute(Float) (- _output_get_2 _output_get))) (Math|Float|Sign(Float) (- _output_get_2 _output_get)))) (LocalVariables|GetDestinationAltitude))) 2.0)
    (Utilities|Time|ClearTimerbyFunctionName self (Variables|Elevetor|GetMoveFunctionTimer))
    (Variables|Elevetor|SetCurrentFloor (Variables|Elevetor|GetTargetedFloor))
    (CallFunction|AtFloor)
    (Transformation|SetRelativeLocation (Variables|Default|GetElevatorFloorCage) (Math|Vector|MakeVector (.x _relativelocation) (.y _relativelocation) (LocalVariables|GetDestinationAltitude)) false false)
    (else
      (Transformation|SetRelativeLocation (Variables|Default|GetElevatorFloorCage) (Math|Vector|MakeVector (.x _relativelocation) (.y _relativelocation) (+ _output_get_3 (* (Math|Float|Clamp(Float) (* (Variables|Elevetor|GetElevatorMaxSpeed) (Variables|Elevetor|GetPositionUpdateRate)) 0.0 (Math|Float|Absolute(Float) (- _output_get_2 _output_get))) (Math|Float|Sign(Float) (- _output_get_2 _output_get))))) false false))))