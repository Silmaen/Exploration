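; BP_Elevator is an interactable elevator actor that raises and lowers its floor cage between a base altitude and an upper height.
; Each Interaction event alternates through a FlipFlop between playing and reversing the ElevatorMovement timeline.
; The timeline's value, scaled by UpAltitude and offset by BaseAltitude, sets the cage's relative Z without sweeping.
; A box-overlap check on the interacting character exists but is left disconnected.
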(event EventInteraction
  (params (CharacterReference :type BP%20EXP%20Pawn%20Object%20Reference))
  (bind _elevatorfloorcage (Variables|Default|GetElevatorFloorCage))
  (bind _relativelocation (Variables|/Script/Engine.SceneComponent|GetRelativeLocation _elevatorfloorcage))
  (Development|PrintString "Elevator commanded")
  (Utilities|FlowControl|FlipFlop
    (:A
      (bind _elevatormovement (Timeline|ElevatorMovement Play)
        (:Update
          (Transformation|SetRelativeLocation _elevatorfloorcage (Math|Vector|MakeVector (.x _relativelocation) (.y _relativelocation) (+ (* _elevatormovement (Variables|Default|GetUpAltitude)) (Variables|Default|GetBaseAltitude))) false false))))
    (:B
      (Timeline|ElevatorMovement Reverse))))

(fn ConstructionScript)