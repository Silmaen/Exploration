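; Right-hand lab door actor that extends a parent door Blueprint with its own swing, handle motion and sign text.
; Opening and handle events call the parent, then rotate the door in yaw and the handle in pitch, scaling each input ratio by a maximum angle.
; The construction script fills the sign with a room number offset by floor in hundreds, plus two additional text lines.
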(event EventSetHandlePosition
  (params (HandleRatio :type Float%20%28single-precision%29))
  (|CallParentFunction HandleRatio)
  (Transformation|SetRelativeRotation (Variables|Default|GetPoignee) (Math|Rotator|MakeRotator 0.0 (* HandleRatio (Variables|State|GetHandleMaxAngle)) 0.0) false false))

(event EventSetDoorOpening
  (params (OpeningPercent :type Float%20%28single-precision%29))
  (|CallParentFunction OpeningPercent)
  (Transformation|SetRelativeRotation (Variables|Default|GetDoor) (Math|Rotator|MakeRotator 0.0 0.0 (* OpeningPercent (Variables|State|GetOpeningAngle))) false false))

(fn ConstructionScript
  (|CallParentFunction)
  (SignScript|SetTexttoSign))

(fn SetTexttoSign
  (Rendering|Components|TextRender|SetText (Variables|Default|GetRoom%20Number) (Utilities|Text|ToText(Integer) (+ (Variables|SignScript|GetRoomNumber) (* (Variables|SignScript|GetFloorNumber) 100)) false true 2 3))
  (Rendering|Components|TextRender|SetText (Variables|Default|GetAdditionnalTextL1) (Variables|SignScript|GetLine1))
  (Rendering|Components|TextRender|SetText (Variables|Default|GetAddtionnalTextL2) (Variables|SignScript|GetLine2)))