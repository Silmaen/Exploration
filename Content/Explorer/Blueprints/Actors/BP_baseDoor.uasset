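; Base door Blueprint whose Interaction event toggles the door between open and closed.
; Leaving the starting state plays an optional handle timeline, then the door timeline unless Locked; returning reverses the door timeline directly, skipping handle and lock.
; StartOpen inverts the opening value and sets the construction-time state.
; SetDoorOpening only updates the Open flag and SetHandlePosition is empty, so this file moves no geometry.
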(event EventInteraction
  (params (CharacterReference :type BP%20EXP%20Pawn%20Object%20Reference))
  (bind _open_ (Variables|State|GetOpen?))
  (bind _startopen_ (Variables|State|GetStartOpen?))
  (if _startopen_
    (if _open_
      (if (Variables|State|GetHasHandleAnimation?) :!label _label
        (bind _movehandle (Timeline|HandleMovement PlayFromStart)
          (:Update
            (State|SetHandlePosition _movehandle))
          (:Finished
            (Utilities|FlowControl|Sequence
              (:then_0
                (Timeline|HandleMovement SetNewTime))
              (:then_1
                (if (not (Variables|State|GetLocked?)) :!label _label_2
                  (bind _dooropen (Timeline|DoorOpeningEvolution Play)
                    (:Update
                      (if _startopen_
                        (State|SetDoorOpening (- 1.0 _dooropen))
                        (else
                          (State|SetDoorOpening _dooropen))))))))))
        (else
          (goto _label_2)))
      (else
        (Timeline|DoorOpeningEvolution Reverse)))
    (elif _open_
      (Timeline|DoorOpeningEvolution Reverse)
      (else
        (goto _label)))))

(fn ConstructionScript
  (State|SetDoorOpening (select (Variables|State|GetStartOpen?) 1.0 0.0)))

(fn SetDoorOpening
  (params (OpeningPercent :type Float%20%28single-precision%29))
  (Variables|State|SetOpen? (!= OpeningPercent 0.0)))

(fn SetHandlePosition
  (params (HandleRatio :type Float%20%28single-precision%29)))