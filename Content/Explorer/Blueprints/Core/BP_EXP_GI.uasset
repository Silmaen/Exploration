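; BP_EXP_GI is the Explorer game instance that carries player state across level changes.
; On Init it creates a BP_EXP_SaveGame object, to which it delegates saving, restoring and printing state, with on-screen debug messages.
; GoToLevel saves the character, sets a Restore flag and opens the named level.
; SetupMode writes the current game mode to BP_EXP_GS and switches input to game only.
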(event EventInit
  (bind _returnvalue (SaveGame|CreateSaveGameObject "/Game/Explorer/Blueprints/Core/BP_EXP_SaveGame.BP_EXP_SaveGame_C"))
  (Variables|Default|SetSaveGame _returnvalue))

(fn SavePlayer
  (params (Character :type BP%20EXP%20Pawn%20Object%20Reference))
  (Default|SavePlayer (Variables|Default|GetSaveGame) Character)
  (bind _returnvalue (Game|GetCurrentLevelName true))
  (Development|PrintString (Utilities|String|Append _returnvalue ": Save State from Game Instance") true true "(R=0.004132,G=0.126115,B=1.000000,A=1.000000)" 1e+01))

(fn RestorePlayer
  (params (Player :type BP%20EXP%20Pawn%20Object%20Reference))
  (Default|RestorePlayer (Variables|Default|GetSaveGame) Player)
  (bind _returnvalue (Game|GetCurrentLevelName true))
  (Development|PrintString (Utilities|String|Append _returnvalue ": Restore State from Game Instance") true true "(R=0.897508,G=0.000000,B=1.000000,A=1.000000)" 1e+01))

(fn GotoLevel
  (params (Character :type BP%20EXP%20Pawn%20Object%20Reference) (LevelName :type Name) (Options :type String) (CurrentGameMode :type E_EXP_GameMode%20Enum :default "NewEnumerator0"))
  (CallFunction|SavePlayer Character)
  (Variables|Default|SetRestore? true)
  (Game|OpenLevel(byName) LevelName false Options))

(fn SetupMode
  (params (CurrentGameMode :type E_EXP_GameMode%20Enum :default "NewEnumerator0"))
  (Utilities|FlowControl|Sequence
    (:then_0
      (Variables|/Game/Explorer/Blueprints/Core/BP_EXP_GS.BP_EXP_GS_C|SetCurrentGameMode (.AsBP%20EXP%20GS (Utilities|Casting|CastToBP_EXP_GS (Game|GetGameState))) CurrentGameMode))
    (:then_1
      (Input|SetInputModeGameOnly (Game|GetPlayerController 0)))))

(fn PrintSave
  (Default|PrintState (Variables|Default|GetSaveGame)))