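; Save game object for the Explorer game that stores the player's health, temperature, stamina and inventory, plus a list of saved level names.
; SavePlayer rebuilds each inventory slot as a new item of the same class owned by the save, copying row name and amount.
; RestorePlayer writes the stats back and imports the inventory into the player's component.
; Level saving records names only, RestoreLevel just warns about unsaved levels, and PrintState dumps player data for debugging.
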(fn SavePlayer
  (params (Player :type BP%20EXP%20Pawn%20Object%20Reference))
  (bind _bp_exp_inventory (Variables|/Game/Explorer/Blueprints/Core/BP_EXP_Pawn.BP_EXP_Pawn_C|GetBP_EXP_Inventory Player))
  (Utilities|FlowControl|Sequence
    (:then_0
      ;[1 1 1] Health
      (Variables|Player|health|SetCurrentHealth (Variables|/Game/Explorer/Blueprints/Core/BP_EXP_Pawn.BP_EXP_Pawn_C|GetCurrentHealth Player))
      (Variables|Player|health|SetMaxHealth (Variables|/Game/Explorer/Blueprints/Core/BP_EXP_Pawn.BP_EXP_Pawn_C|GetMaxHealth Player)))
    (:then_1
      ;[1 1 1] Temperature
      (Variables|Player|Temperature|SetClothingTempModifier (Variables|/Game/Explorer/Blueprints/Core/BP_EXP_Pawn.BP_EXP_Pawn_C|GetClothingTempModifier Player))
      (Variables|Player|Temperature|SetBodyTemp (Variables|/Game/Explorer/Blueprints/Core/BP_EXP_Pawn.BP_EXP_Pawn_C|GetBodyTemp Player)))
    (:then_2
      ;[1 1 1] Stamina
      (Variables|Player|Stamina|SetMaxStamina (Variables|/Game/Explorer/Blueprints/Core/BP_EXP_Pawn.BP_EXP_Pawn_C|GetMaxStamina Player))
      (Variables|Player|Stamina|SetCurrentStamina (Variables|/Game/Explorer/Blueprints/Core/BP_EXP_Pawn.BP_EXP_Pawn_C|GetCurrentStamina Player))
      (Variables|Player|Stamina|SetOutOfBreath? (Variables|/Game/Explorer/Blueprints/Core/BP_EXP_Pawn.BP_EXP_Pawn_C|GetOutOfBreath? Player)))
    (:then_3
      ;[1 1 1] Inventory
      (Utilities|Array|Clear (Variables|Player|Inventory|GetInventory))
      (for _index (range 0 (- (Variables|/Game/Explorer/Blueprints/Components/BP_EXP_InventoryComponent.BP_EXP_InventoryComponent_C|GetSlots _bp_exp_inventory) 1))
        (bind _returnvalue (Game|ConstructObjectfromClass (Utilities|GetClass (Utilities|Array|Get(acopy) (Default|GetInventory _bp_exp_inventory) _index)) self))
        (Utilities|Array|Add (Variables|Player|Inventory|GetInventory) _returnvalue)
        (Utilities|IsValid (Utilities|Array|Get(acopy) (Default|GetInventory _bp_exp_inventory) _index)
          (:Is%20Valid
            (if (!= (Utilities|GetClass (Utilities|Array|Get(acopy) (Default|GetInventory _bp_exp_inventory) _index)) "/Game/Explorer/Blueprints/Inventory/Objects/BP_EXP_InvItem_Empty.BP_EXP_InvItem_Empty_C")
              (Variables|/Game/Explorer/Blueprints/Inventory/Objects/BP_EXP_InventoryItem.BP_EXP_InventoryItem_C|SetRowName _returnvalue (Variables|/Game/Explorer/Blueprints/Inventory/Objects/BP_EXP_InventoryItem.BP_EXP_InventoryItem_C|GetRowName (Utilities|Array|Get(acopy) (Default|GetInventory _bp_exp_inventory) _index)))
              (Default|SetAmount _returnvalue (Default|GetAmount (Utilities|Array|Get(acopy) (Default|GetInventory _bp_exp_inventory) _index))))))))))

(fn RestorePlayer
  (params (Player :type BP%20EXP%20Pawn%20Object%20Reference))
  (Utilities|FlowControl|Sequence
    (:then_0
      ;[1 1 1] Health
      (Variables|/Game/Explorer/Blueprints/Core/BP_EXP_Pawn.BP_EXP_Pawn_C|SetCurrentHealth Player (Variables|Player|health|GetCurrentHealth))
      (Variables|/Game/Explorer/Blueprints/Core/BP_EXP_Pawn.BP_EXP_Pawn_C|SetMaxHealth Player (Variables|Player|health|GetMaxHealth)))
    (:then_1
      ;[1 1 1] Temperature
      (Variables|/Game/Explorer/Blueprints/Core/BP_EXP_Pawn.BP_EXP_Pawn_C|SetClothingTempModifier Player (Variables|Player|Temperature|GetClothingTempModifier))
      (Variables|/Game/Explorer/Blueprints/Core/BP_EXP_Pawn.BP_EXP_Pawn_C|SetBodyTemp Player (Variables|Player|Temperature|GetBodyTemp)))
    (:then_2
      ;[1 1 1] Stamina
      (Variables|/Game/Explorer/Blueprints/Core/BP_EXP_Pawn.BP_EXP_Pawn_C|SetMaxStamina Player (Variables|Player|Stamina|GetMaxStamina))
      (Variables|/Game/Explorer/Blueprints/Core/BP_EXP_Pawn.BP_EXP_Pawn_C|SetCurrentStamina Player (Variables|Player|Stamina|GetCurrentStamina))
      (Variables|/Game/Explorer/Blueprints/Core/BP_EXP_Pawn.BP_EXP_Pawn_C|SetOutOfBreath? Player (Variables|Player|Stamina|GetOutOfBreath?)))
    (:then_3
      ;[1 1 1] Inventory
      (Default|ImportValue (Variables|/Game/Explorer/Blueprints/Core/BP_EXP_Pawn.BP_EXP_Pawn_C|GetBP_EXP_Inventory Player) (Variables|Player|Inventory|GetInventory)))))

(fn PrintState
  (Development|PrintString 0 (Utilities|String|Append "Health: " (Utilities|String|ToString(Float) (Variables|Player|health|GetCurrentHealth)) " / " (Utilities|String|ToString(Float) (Variables|Player|health|GetMaxHealth))) true true "(R=0.000000,G=0.660000,B=1.000000,A=1.000000)" 5.0)
  (Development|PrintString 0 (Utilities|String|Append "Temp: " (Utilities|String|ToString(Float) (Variables|Player|Temperature|GetBodyTemp)) "Modifier" (Utilities|String|ToString(Float) (Variables|Player|Temperature|GetClothingTempModifier))) true true "(R=0.000000,G=0.660000,B=1.000000,A=1.000000)" 5.0)
  (Development|PrintString 0 (Utilities|String|Append "Stamina: " (Utilities|String|ToString(Float) (Variables|Player|Stamina|GetCurrentStamina)) " / " (Utilities|String|ToString(Float) (Variables|Player|Stamina|GetMaxStamina)) " oob: " (Utilities|String|ToString(Boolean) (Variables|Player|Stamina|GetOutOfBreath?))) true true "(R=0.000000,G=0.660000,B=1.000000,A=1.000000)" 5.0)
  (for (_array_element _array_index) (Variables|Player|Inventory|GetInventory)
    (Development|PrintString 0 (Utilities|String|Append (Utilities|String|ToString(Integer) _array_index) " " (Utilities|String|ToString(Text) (.name (.iteminfo (Default|GetInventoryItemInfo _array_element)))) " " (Utilities|String|ToString(Integer) (Default|GetAmount _array_element))) true true "(R=0.000000,G=0.660000,B=1.000000,A=1.000000)" 5.0)))

(fn SaveLevel
  (params (LevelName :type String))
  (if (not (Level|IsLevelSaved LevelName))
    (Utilities|Array|Add (Variables|Levels|GetSavedLevels) LevelName)))

(fn RestoreLevel
  (params (LevelName :type String))
  (if (not (Level|IsLevelSaved LevelName))
    (Development|PrintString 0 (Utilities|String|Append "try to restore level '" LevelName "' but not saved"))))

(fn IsLevelSaved
  (params (LevelName :type String))
  (return (Utilities|Array|ContainsItem (Variables|Levels|GetSavedLevels) LevelName)))