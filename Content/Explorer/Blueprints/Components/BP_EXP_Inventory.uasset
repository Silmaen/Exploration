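; Inventory component for the Explorer game that holds a fixed number of slots as item objects, filled with empty placeholder items on BeginPlay.
; AddItem requires a free slot, then tops up a matching stackable item and puts any overflow in a new instance in the first empty slot.
; As written, it has no branch that places an item lacking an existing stack with room.
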(event EventBeginPlay
  (CallFunction|IntitializeInventory))

(fn GetInventory
  (return (Variables|Default|GetInventory)))

(fn IntitializeInventory
  (Utilities|Array|Clear (Variables|Default|GetInventory))
  (for _index (range 0 (- (Variables|Default|GetSlots) 1))
    (bind _returnvalue (Game|ConstructObjectfromClass "/Game/Explorer/Blueprints/Inventory/Objects/BP_EXP_InvItem_Empty.BP_EXP_InvItem_Empty_C" self))
    (Utilities|Array|Add (Variables|Default|GetInventory) _returnvalue)))

(fn AddItem
  (params (ItemToAdd :type BP%20EXP%20Inventory%20Item%20Class%20Reference) (AmountToAdd :type Integer))
  (bind (_hasspace _openspaces) (CallFunction|HasSpaceinInventory))
  (LocalVariables|SetL_Class ItemToAdd)
  (LocalVariables|SetL_Amount AmountToAdd)
  (if _hasspace
    (LocalVariables|SetL_OpenSpaces _openspaces)
    (for _array_element (Variables|Default|GetInventory)
      (if (== (Utilities|GetClass _array_element) (LocalVariables|GetL_Class))
        (bind _output_get (LocalVariables|SetL_Item _array_element))
        (if (Default|GetCanStack _output_get)
          (if (> (Default|GetRoomOnstack (LocalVariables|GetL_Item)) 0)
            (if (<= (+ (Default|GetAmount (LocalVariables|GetL_Item)) (LocalVariables|GetL_Amount)) (Default|GetMaxStackAmount (LocalVariables|GetL_Item)))
              (Default|SetAmount (LocalVariables|GetL_Item) (+ (Default|GetAmount (LocalVariables|GetL_Item)) (LocalVariables|GetL_Amount)))
              (return true)
              (elif (> (LocalVariables|GetL_OpenSpaces) 0)
                (LocalVariables|SetL_Amount (- (LocalVariables|GetL_Amount) (Default|GetRoomOnstack (LocalVariables|GetL_Item))))
                (Default|SetAmount (LocalVariables|GetL_Item) (Default|GetMaxStackAmount (LocalVariables|GetL_Item)))
                (else
                  (return false)))))))
      (bind (_array_element_2 _array_index) (Utilities|Array|ForEachLoopwithBreak (Variables|Default|GetInventory) :!label _label)
        (:LoopBody
          (if (== (Utilities|GetClass _array_element_2) "/Game/Explorer/Blueprints/Inventory/Objects/BP_EXP_InvItem_Empty.BP_EXP_InvItem_Empty_C")
            (LocalVariables|SetL_index _array_index)
            (goto _label Break)
            (else
              (LocalVariables|SetL_index -1))))
        (:Completed
          (if (>= (LocalVariables|GetL_index) 0)
            (bind _returnvalue (Game|ConstructObjectfromClass (LocalVariables|GetL_Class) self))
            (Default|SetAmount _returnvalue (LocalVariables|GetL_Amount))
            (Utilities|Array|SetArrayElem (Variables|Default|GetInventory) (LocalVariables|GetL_index) _returnvalue)
            (return true)
            (else
              (return false))))))
    (else
      (return false))))

(fn HasSpaceinInventory
  (bind _l_openspace (LocalVariables|GetL_OpenSpace))
  (for _array_element (Variables|Default|GetInventory)
    (if (== (Utilities|GetClass _array_element) "/Game/Explorer/Blueprints/Inventory/Objects/BP_EXP_InvItem_Empty.BP_EXP_InvItem_Empty_C")
      (Math|Integer|IncrementInt _l_openspace)))
  (return (> _l_openspace 0) _l_openspace))