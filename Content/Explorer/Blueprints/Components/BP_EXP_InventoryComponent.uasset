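; Explorer inventory component that holds a fixed number of slots as item objects, pre-filled with empty-item placeholders on BeginPlay.
; AddItem requires a free slot, then tops up a matching stack and puts overflow into a new item in the first empty slot.
; Slot getters and setters support swapping items between inventories.
; ImportValue rebuilds the slots from another item array, copying class, row name and amount.
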(event EventBeginPlay
  (CallFunction|InitializeInventory))

(fn GetInventory
  (return (Variables|Default|GetInventory)))

(fn InitializeInventory
  (Utilities|Array|Clear (Variables|Default|GetInventory))
  (for _index (range 0 (- (Variables|Default|GetSlots) 1))
    (bind _returnvalue (Game|ConstructObjectfromClass "/Game/Explorer/Blueprints/Inventory/Objects/BP_EXP_InvItem_Empty.BP_EXP_InvItem_Empty_C" self))
    (Utilities|Array|Add (Variables|Default|GetInventory) _returnvalue)))

(fn AddItem
  (params (ItemToAdd :type BP%20EXP%20Inventory%20Item%20Class%20Reference) (AmountToAdd :type Integer))
  (bind (_hasspace _openspaces) (CallFunction|HasSpaceinInventory))
  (LocalVariables|SetL_Class ItemToAdd)
  (LocalVariables|SetL_Amount AmountToAdd)
  (if _hasspace
    (LocalVariables|SetL_OpenSpaces _openspaces)
    (for _array_element (Variables|Default|GetInventory)
      (if (== (Utilities|GetClass _array_element) (LocalVariables|GetL_Class))
        (bind _output_get (LocalVariables|SetL_Item _array_element))
        (if (Default|GetCanStack _output_get)
          (if (> (Default|GetRoomOnstack (LocalVariables|GetL_Item)) 0)
            (if (<= (+ (Default|GetAmount (LocalVariables|GetL_Item)) (LocalVariables|GetL_Amount)) (Default|GetMaxStackAmount (LocalVariables|GetL_Item)))
              (Default|SetAmount (LocalVariables|GetL_Item) (+ (Default|GetAmount (LocalVariables|GetL_Item)) (LocalVariables|GetL_Amount)))
              (return true)
              (elif (> (LocalVariables|GetL_OpenSpaces) 0)
                (LocalVariables|SetL_Amount (- (LocalVariables|GetL_Amount) (Default|GetRoomOnstack (LocalVariables|GetL_Item))))
                (Default|SetAmount (LocalVariables|GetL_Item) (Default|GetMaxStackAmount (LocalVariables|GetL_Item)))
                (else
                  (return false)))))))
      (bind (_array_element_2 _array_index) (Utilities|Array|ForEachLoopwithBreak (Variables|Default|GetInventory) :!label _label)
        (:LoopBody
          (if (== (Utilities|GetClass _array_element_2) "/Game/Explorer/Blueprints/Inventory/Objects/BP_EXP_InvItem_Empty.BP_EXP_InvItem_Empty_C")
            (LocalVariables|SetL_index _array_index)
            (goto _label Break)
            (else
              (LocalVariables|SetL_index -1))))
        (:Completed
          (if (>= (LocalVariables|GetL_index) 0)
            (bind _returnvalue (Game|ConstructObjectfromClass (LocalVariables|GetL_Class) self))
            (Default|SetAmount _returnvalue (LocalVariables|GetL_Amount))
            (Utilities|Array|SetArrayElem (Variables|Default|GetInventory) (LocalVariables|GetL_index) _returnvalue)
            (return true)
            (else
              (return false))))))
    (else
      (return false))))

(fn HasSpaceinInventory
  (bind _l_openspace (LocalVariables|GetL_OpenSpace))
  (for _array_element (Variables|Default|GetInventory)
    (if (== (Utilities|GetClass _array_element) "/Game/Explorer/Blueprints/Inventory/Objects/BP_EXP_InvItem_Empty.BP_EXP_InvItem_Empty_C")
      (Math|Integer|IncrementInt _l_openspace)))
  (return (> _l_openspace 0) _l_openspace))

(fn SetSlotinInventory
  (params (Item :type BP%20EXP%20Inventory%20Item%20Object%20Reference) (Index :type Integer))
  (bind _inventory (Variables|Default|GetInventory))
  (if (<= Index (Utilities|Array|LastIndex _inventory))
    (Utilities|Array|SetArrayElem _inventory Index Item)
    (return true)
    (else
      (return false))))

(fn SwapItems
  (params (FromInventory :type BP%20EXP%20Inventory%20Component%20Object%20Reference) (FromIndex :type Integer) (ToInventory :type BP%20EXP%20Inventory%20Component%20Object%20Reference) (ToIndex :type Integer))
  (bind _output_get (LocalVariables|SetL_FromItem (CallFunction|GetIteminSlot FromInventory FromIndex)))
  (bind _output_get_2 (LocalVariables|SetL_ToItem (CallFunction|GetIteminSlot ToInventory ToIndex)))
  (CallFunction|SetSlotinInventory FromInventory _output_get_2 FromIndex)
  (CallFunction|SetSlotinInventory ToInventory _output_get ToIndex))

(fn GetIteminSlot
  (params (Index :type Integer))
  (bind _inventory (Variables|Default|GetInventory))
  (bind _output (Utilities|Array|Get(acopy) _inventory Index))
  (Utilities|IsValid _output
    (:Is%20Valid
      (return _output))
    (:Is%20Not%20Valid
      (return 0))))

(fn ImportValue
  (params (Invent :type Array%20of%20BP%20EXP%20Inventory%20Item%20Object%20References))
  (Variables|Default|SetSlots (Utilities|Array|Length Invent))
  (Utilities|Array|Clear (Variables|Default|GetInventory))
  (for _array_element Invent
    (bind _returnvalue (Game|ConstructObjectfromClass (Utilities|GetClass _array_element) self))
    (Utilities|Array|Add (Variables|Default|GetInventory) _returnvalue)
    (Variables|/Game/Explorer/Blueprints/Inventory/Objects/BP_EXP_InventoryItem.BP_EXP_InventoryItem_C|SetRowName _returnvalue (Variables|/Game/Explorer/Blueprints/Inventory/Objects/BP_EXP_InventoryItem.BP_EXP_InventoryItem_C|GetRowName _array_element))
    (Default|SetAmount _returnvalue (Default|GetAmount _array_element))))